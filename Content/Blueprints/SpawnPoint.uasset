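; Enemy spawn point that, once activated by Opened, spawns wandering AI enemies at its Cube's location during timed bursts.
; A BeginPlay loop checks the Rounds actor's wave state and spawn number, waiting longer with more HeistData hostages.
; Each burst calls WaveCount on Rounds, raises HitPoints and toggles TheyreAlive to gate a once-per-second spawn loop.
; The Spawn interval grows every cycle, even when idle, until it passes a cap and cycling stops.
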(event Custom|SpawnThem
  (if (Variables|Default|GetThey'reAlive) :!label _label
    (Game|SpawnActorfromClass "/Game/Yash/Blueprint/AI/Enemy_Wanderer/EnemyAI_Wanderer.EnemyAI_Wanderer_C" (Math|Conversions|ToTransform(Vector) (Transformation|GetWorldLocation (Variables|Default|GetCube))) "AdjustIfPossibleButDontSpawnIfColliding" 0 0))
  (Utilities|FlowControl|Delay 1.0)
  (goto _label))

(event Custom|Opened
  (Variables|Default|SetActiveSpawn true))

(event EventBeginPlay
  (Utilities|FlowControl|Delay 2.0)
  (bind _asheist_data (Utilities|Casting|CastToHeistData (Game|GetGameInstance) :!label _label))
  (if (Variables|Default|GetActiveSpawn)
    (bind _outactors (Actor|GetAllActorsOfClass "/Game/Blueprints/Rounds.Rounds_C"))
    (bind _asrounds (Utilities|Casting|CastToRounds (Utilities|Array|Get(acopy) _outactors)))
    (if (Variables|/Game/Blueprints/Rounds.Rounds_C|GetWaveIncrease _asrounds)
      (if (<= (Variables|/Game/Blueprints/Rounds.Rounds_C|GetSpawnNumber _asrounds) 10)
        (Utilities|FlowControl|Delay (+ (Math|Conversions|ToFloat(Integer) (Variables|/Game/Blueprints/HeistData.HeistData_C|GetHostages _asheist_data)) 2.0) :!label _label_2)
        (bind _outactors_2 (Actor|GetAllActorsOfClass "/Game/Blueprints/Rounds.Rounds_C"))
        (Variables|Default|SetHitPoints (+ (Variables|Default|GetHitPoints) 1.0))
        (Default|WaveCount _outactors_2)
        (Variables|Default|SetThey'reAlive true)
        (CallFunction|SpawnThem)
        (Utilities|FlowControl|Delay (Variables|Default|GetSpawn))
        (Variables|Default|SetThey'reAlive false)
        (if (<= (Variables|Default|GetSpawn) 1e+01)
          (Variables|Default|SetSpawn (+ (Variables|Default|GetSpawn) 0.05))
          (goto _label))
        (else
          (Utilities|FlowControl|Delay (+ (Math|Conversions|ToFloat(Integer) (Variables|/Game/Blueprints/HeistData.HeistData_C|GetHostages _asheist_data)) 2.0) :!label _label_3)
          (Utilities|FlowControl|Delay (Variables|Default|GetSpawn))
          (if (<= (Variables|Default|GetSpawn) 1e+01)
            (Variables|Default|SetSpawn (+ (Variables|Default|GetSpawn) 0.05))
            (goto _label))))
      (elif (<= (Variables|/Game/Blueprints/Rounds.Rounds_C|GetSpawnNumber _asrounds) 0)
        (goto _label_2)
        (else
          (goto _label_3))))
    (else
      (goto _label_3))))

(fn ConstructionScript)