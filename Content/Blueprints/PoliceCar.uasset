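; Police car Blueprint that plays a scripted pull-up animation when play begins.
; Chained MoveComponentTo calls snap the body cube to an offset, slide it back to origin with a slight rotation, then quickly level it.
; A parallel Delay loop spins two wheel cylinders, entered only if PullingUp is set.
; Arrival clears PullingUp, but the running loop never rechecks it, so the wheels keep turning.
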(event Custom|OnTheMove
  (if (Variables|Default|GetPullingUp)
    (bind _output_get (Variables|Default|SetWheels (+ (Variables|Default|GetWheels) 1.0) :!label _label))
    (Transformation|SetRelativeRotation (Variables|Default|GetCylinder) (Math|Rotator|MakeRotator 9e+01 _output_get 0.0) false false)
    (Utilities|FlowControl|Delay 0.01)
    (goto _label)))

(event Custom|Arrived
  (Variables|Default|SetPullingUp false))

(event EventBeginPlay
  (bind _cube (Variables|Default|GetCube))
  (CallFunction|OntheMove)
  (Components|MoveComponentTo _cube "5000.000000, 0, 0" "0, 0, 0" false false 0.0 false)
  (Components|MoveComponentTo _cube "0.000000, 0, 0" "4.000000, 0, 0" false false 3.0 false)
  (Components|MoveComponentTo _cube "0, 0, 0" "0.000000, 0, 0" false false 0.3 false)
  (CallFunction|Arrived))

(fn ConstructionScript)