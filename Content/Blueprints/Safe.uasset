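; Safe actor that the player cracks with either a drill or a bomb to release a money bag.
; The Door event reads the character's DrillBomb mode to spawn a one-time Drill beside the safe, or spend a bomb, show Cube2 and trigger BlownOpen after a delay.
; BlownOpen fires particles, while both it and BrokenOpen, which is not called within this graph, spawn a MoneyBag and swing Cube1 open.
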(event Custom|BlownOpen
  (Components|Activation|SetActive (Variables|Default|GetParticleSystem) true false)
  (Rendering|SetVisibility (Variables|Default|GetCube2) false false)
  (Game|SpawnActorfromClass "/Game/Blueprints/MoneyBag.MoneyBag_C" (Transformation|GetActorTransform) "AdjustIfPossibleButAlwaysSpawn" 0 0)
  (Components|MoveComponentTo (Variables|Default|GetCube1) "-65.000000,-60.000000,15.000000" "0,110.000000, 0" false false 0.2 true))

(event Custom|BrokenOpen
  (Game|SpawnActorfromClass "/Game/Blueprints/MoneyBag.MoneyBag_C" (Transformation|GetActorTransform) "AdjustIfPossibleButAlwaysSpawn" 0 0)
  (Components|MoveComponentTo (Variables|Default|GetCube1) "-65.000000,-60.000000,15.000000" "0,110.000000, 0" false false 1.0 true))

(event EventDoor
  (bind _returnvalue (Transformation|GetActorTransform))
  (bind _asfirst_person_character (Utilities|Casting|CastToFirstPersonCharacter (Game|GetPlayerCharacter 0)))
  (switch int (Variables|/Game/FirstPersonBP/Blueprints/FirstPersonCharacter.FirstPersonCharacter_C|GetDrill/Bomb _asfirst_person_character)
    (:0
      (Utilities|FlowControl|DoOnce false
        (:Completed
          (Game|SpawnActorfromClass "/Game/Blueprints/Drill.Drill_C" (Math|Transform|MakeTransform (Math|Vector|MakeVector (- (.x (.location _returnvalue)) 1.2e+02) (.y (.location _returnvalue)) (.z (.location _returnvalue))) (.rotation _returnvalue) "1.200000,1.200000,1.200000") "Undefined" 0 0))))
    (:1
      (if (>= (Variables|/Game/FirstPersonBP/Blueprints/FirstPersonCharacter.FirstPersonCharacter_C|GetBomb _asfirst_person_character) 1)
        (Variables|/Game/FirstPersonBP/Blueprints/FirstPersonCharacter.FirstPersonCharacter_C|SetBomb _asfirst_person_character (- (Variables|/Game/FirstPersonBP/Blueprints/FirstPersonCharacter.FirstPersonCharacter_C|GetBomb _asfirst_person_character) 1))
        (Rendering|SetVisibility (Variables|Default|GetCube2) true false)
        (Utilities|FlowControl|Delay 2.0)
        (CallFunction|BlownOpen)))))

(fn ConstructionScript)