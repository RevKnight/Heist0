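; Heist exit zone that lets a first-person player who is carrying something escape and earn money.
; Overlapping the box shows an Exit progress widget driven by a short-delay loop, which resets and removes it if the player leaves.
; A full timer adds a random cash reward to the HeistData game instance and calls its Finished function.
; A level-reload branch is present but disconnected.
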(event OnComponentBeginOverlap(Box)
  (params (OverlappedComponent :type Primitive%20Component%20Object%20Reference) (OtherActor :type Actor%20Object%20Reference) (OtherComp :type Primitive%20Component%20Object%20Reference) (OtherBodyIndex :type Integer) (bFromSweep :type Boolean) (SweepResult :type Hit%20Result%20Structure%20%28by%20ref%29))
  (bind _asfirst_person_character (Utilities|Casting|CastToFirstPersonCharacter OtherActor))
  (if (Variables|/Game/FirstPersonBP/Blueprints/FirstPersonCharacter.FirstPersonCharacter_C|GetCarrying _asfirst_person_character)
    (Variables|Default|SetLeaving true)
    (bind _returnvalue (UserInterface|CreateWidget "/Game/Exit.Exit_C"))
    (UserInterface|Viewport|AddtoPlayerScreen _returnvalue)
    (if (Variables|Default|GetLeaving) :!label _label
      (bind _output_get (Variables|Default|SetTimeToExit (+ (Variables|Default|GetTimeToExit) 0.01)))
      (Variables|/Game/Exit.Exit_C|SetPercentage _returnvalue _output_get)
      (Utilities|FlowControl|Delay 0.01)
      (if (<= _output_get 1.0)
        (goto _label)
        (else
          (bind _asheist_data (Utilities|Casting|CastToHeistData (Game|GetGameInstance)))
          (Variables|/Game/Blueprints/HeistData.HeistData_C|SetCashFollow _asheist_data (+ (Variables|/Game/Blueprints/HeistData.HeistData_C|GetCashFollow _asheist_data) (Math|Random|RandomIntegerinRange 4000 5000)))
          (Default|Finished _asheist_data)
          (Development|PrintString "Money Earned" true true "(R=0.000000,G=0.660000,B=1.000000,A=1.000000)" 5.0)
          (Development|PrintString "Exited" true true "(R=0.000000,G=0.660000,B=1.000000,A=1.000000)" 5.0)))
      (else
        (Variables|Default|SetTimeToExit 0.0)
        (Widget|RemovefromParent _returnvalue)))))

(event OnComponentEndOverlap(Box)
  (params (OverlappedComponent :type Primitive%20Component%20Object%20Reference) (OtherActor :type Actor%20Object%20Reference) (OtherComp :type Primitive%20Component%20Object%20Reference) (OtherBodyIndex :type Integer))
  (Utilities|Casting|CastToFirstPersonCharacter OtherActor)
  (Variables|Default|SetLeaving false))

(fn ConstructionScript)