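; Weapon pickup actor that shows a Micro Uzi, M416, AKS-74U or Benelli mesh chosen by GunNumber on BeginPlay.
; Its Door event swaps this gun into the first-person character's inventory, hides it and destroys it after a delay.
; The previously held gun respawns at the character's Arrow6 as a Dropped WeaponTest.
; Non-dropped pickups also set MachineGunTotal based on that previous gun, except for the Benelli.
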(event EventBeginPlay
  (bind _skeletalmesh (Variables|Default|GetSkeletalMesh))
  (Utilities|FlowControl|Delay 0.05)
  (switch int (Variables|Default|GetGunNumber)
    (:0
      (Class|SkinnedMeshComponent|SetSkeletalMesh _skeletalmesh "/Game/Weapons/Meshes/Weapons/SKM_MicroUzi.SKM_MicroUzi" true))
    (:2
      (Class|SkinnedMeshComponent|SetSkeletalMesh _skeletalmesh "/Game/Weapons/Meshes/Weapons/SKM_M416.SKM_M416" true))
    (:4
      (Class|SkinnedMeshComponent|SetSkeletalMesh _skeletalmesh "/Game/Weapons/Meshes/Weapons/SKM_AKS74U.SKM_AKS74U" true))
    (:6
      (Class|SkinnedMeshComponent|SetSkeletalMesh _skeletalmesh "/Game/Weapons/Meshes/Weapons/SKM_Benelli.SKM_Benelli" true))))

(event EventDoor
  (bind _cube (Variables|Default|GetCube))
  (bind _asfirst_person_character (Utilities|Casting|CastToFirstPersonCharacter (Game|GetPlayerCharacter 0)))
  (Utilities|FlowControl|Sequence
    (:then_0
      (switch int (Variables|/Game/FirstPersonBP/Blueprints/FirstPersonCharacter.FirstPersonCharacter_C|GetGunInventory _asfirst_person_character)
        (:0
          (Utilities|FlowControl|Delay 0.5)
          (if (Variables|Default|GetDropped)
            _
            (else
              (Variables|/Game/FirstPersonBP/Blueprints/FirstPersonCharacter.FirstPersonCharacter_C|SetMachineGunTotal _asfirst_person_character (+ (Variables|/Game/FirstPersonBP/Blueprints/FirstPersonCharacter.FirstPersonCharacter_C|GetSubMachineGunTotal _asfirst_person_character) 25))))
          (bind _returnvalue (Game|SpawnActorfromClass "WeaponTest_C" (Transformation|GetWorldTransform (Variables|/Game/FirstPersonBP/Blueprints/FirstPersonCharacter.FirstPersonCharacter_C|GetArrow6 _asfirst_person_character)) "Undefined" 0 0))
          (Variables|WeaponTest_C|SetGunNumber _returnvalue 0)
          (Variables|WeaponTest_C|SetDropped _returnvalue true))
        (:2
          (Utilities|FlowControl|Delay 0.5)
          (if (Variables|Default|GetDropped)
            _
            (else
              (Variables|/Game/FirstPersonBP/Blueprints/FirstPersonCharacter.FirstPersonCharacter_C|SetMachineGunTotal _asfirst_person_character (+ (Variables|/Game/FirstPersonBP/Blueprints/FirstPersonCharacter.FirstPersonCharacter_C|GetMachineGunTotal _asfirst_person_character) 30))))
          (bind _returnvalue_2 (Game|SpawnActorfromClass "WeaponTest_C" (Transformation|GetWorldTransform (Variables|/Game/FirstPersonBP/Blueprints/FirstPersonCharacter.FirstPersonCharacter_C|GetArrow6 _asfirst_person_character)) "Undefined" 0 0))
          (Variables|WeaponTest_C|SetGunNumber _returnvalue_2 2)
          (Variables|WeaponTest_C|SetDropped _returnvalue_2 true))
        (:4
          (Utilities|FlowControl|Delay 0.5)
          (if (Variables|Default|GetDropped)
            _
            (else
              (Variables|/Game/FirstPersonBP/Blueprints/FirstPersonCharacter.FirstPersonCharacter_C|SetMachineGunTotal _asfirst_person_character (+ (Variables|/Game/FirstPersonBP/Blueprints/FirstPersonCharacter.FirstPersonCharacter_C|GetMachineGunTotal _asfirst_person_character) 30))))
          (bind _returnvalue_3 (Game|SpawnActorfromClass "WeaponTest_C" (Transformation|GetWorldTransform (Variables|/Game/FirstPersonBP/Blueprints/FirstPersonCharacter.FirstPersonCharacter_C|GetArrow6 _asfirst_person_character)) "Undefined" 0 0))
          (Variables|WeaponTest_C|SetGunNumber _returnvalue_3 4)
          (Variables|WeaponTest_C|SetDropped _returnvalue_3 true))
        (:6
          (Utilities|FlowControl|Delay 0.5)
          (bind _returnvalue_4 (Game|SpawnActorfromClass "WeaponTest_C" (Transformation|GetWorldTransform (Variables|/Game/FirstPersonBP/Blueprints/FirstPersonCharacter.FirstPersonCharacter_C|GetArrow6 _asfirst_person_character)) "Undefined" 0 0))
          (Variables|WeaponTest_C|SetGunNumber _returnvalue_4 6)
          (Variables|WeaponTest_C|SetDropped _returnvalue_4 true))))
    (:then_1
      (Variables|/Game/FirstPersonBP/Blueprints/FirstPersonCharacter.FirstPersonCharacter_C|SetGunInventory _asfirst_person_character (Variables|Default|GetGunNumber))
      (Default|SwitchedWeapons _asfirst_person_character)
      (Rendering|SetVisibility (Variables|Default|GetSkeletalMesh) false false)
      (Physics|SetSimulatePhysics _cube false)
      (Collision|SetCollisionEnabled _cube "NoCollision")
      (Utilities|FlowControl|Delay 0.6)
      (Actor|DestroyActor))))

(fn ConstructionScript)