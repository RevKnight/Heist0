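; Heist getaway helicopter that serves as the money drop-off and extraction point, with looping rotor spin, arrival motion and sound.
; Box1 banks earned MoneyBags; Box banks the player's carried bag and loose cash.
; Once the quota is met, staying in Box fills an Exit widget through a Delay loop.
; Completion triggers the fly-away camera sequence, resets HeistData gear and progress, shows JobComplete and pauses the game.
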(event OnComponentBeginOverlap(Box)
  (params (OverlappedComponent :type Primitive%20Component%20Object%20Reference) (OtherActor :type Actor%20Object%20Reference) (OtherComp :type Primitive%20Component%20Object%20Reference) (OtherBodyIndex :type Integer) (bFromSweep :type Boolean) (SweepResult :type Hit%20Result%20Structure%20%28by%20ref%29))
  (bind _asfirst_person_character (Utilities|Casting|CastToFirstPersonCharacter OtherActor))
  (if (Variables|/Game/FirstPersonBP/Blueprints/FirstPersonCharacter.FirstPersonCharacter_C|GetCarrying _asfirst_person_character)
    (bind _output_get (Variables|Default|SetMoneyGained (+ 5000 (Variables|Default|GetMoneyGained))))
    (Variables|Default|SetHelicopterMoney _output_get)
    (bind _returnvalue (Game|SpawnActorfromClass "/Game/Blueprints/MoneyBag.MoneyBag_C" (Transformation|GetWorldTransform (Variables|/Game/FirstPersonBP/Blueprints/FirstPersonCharacter.FirstPersonCharacter_C|GetArrow6 _asfirst_person_character)) "Undefined" 0 0))
    (Variables|/Game/Blueprints/MoneyBag.MoneyBag_C|SetEarned _returnvalue false)
    (bind _returnvalue_2 (UserInterface|CreateWidget "/Game/Widgets/MoneyEarned.MoneyEarned_C"))
    (Variables|/Game/Widgets/MoneyEarned.MoneyEarned_C|SetCash _returnvalue_2 5000)
    (UserInterface|Viewport|AddtoViewport _returnvalue_2 0)
    (Variables|/Game/FirstPersonBP/Blueprints/FirstPersonCharacter.FirstPersonCharacter_C|SetCarrying _asfirst_person_character false)
    (Variables|/Script/Engine.CharacterMovementComponent|SetMaxWalkSpeed (Variables|/Script/Engine.Character|GetCharacterMovement _asfirst_person_character) 6e+02))
  (Variables|Default|SetMoneyGained (+ (Variables|Default|GetMoneyGained) (Variables|/Game/FirstPersonBP/Blueprints/FirstPersonCharacter.FirstPersonCharacter_C|GetMoneyTemp _asfirst_person_character)))
  (Variables|/Game/FirstPersonBP/Blueprints/FirstPersonCharacter.FirstPersonCharacter_C|SetMoneyTemp _asfirst_person_character 0)
  (if (>= (Variables|Default|GetMoneyGained) (Variables|Default|GetMoneyNeeded))
    (Variables|Default|SetLeaving true)
    (bind _returnvalue_3 (UserInterface|CreateWidget "/Game/Widgets/Exit.Exit_C"))
    (UserInterface|Viewport|AddtoPlayerScreen _returnvalue_3)
    (if (Variables|Default|GetLeaving) :!label _label
      (bind _output_get_2 (Variables|Default|SetTimeToExit (+ (Variables|Default|GetTimeToExit) 0.01)))
      (Variables|/Game/Widgets/Exit.Exit_C|SetPercentage _returnvalue_3 _output_get_2)
      (Utilities|FlowControl|Delay 0.05)
      (if (<= _output_get_2 1.0)
        (goto _label)
        (else
          (Utilities|FlowControl|DoOnce false
            (:Completed
              (CallFunction|Flying)
              (bind _asheist_data (Utilities|Casting|CastToHeistData (Game|GetGameInstance)))
              (bind _returnvalue_4 (UserInterface|CreateWidget "/Game/Widgets/MoneyEarned.MoneyEarned_C"))
              (Variables|/Game/Widgets/MoneyEarned.MoneyEarned_C|SetCash _returnvalue_4 (Variables|Default|GetMoneyGained))
              (Variables|/Game/Blueprints/HeistData.HeistData_C|SetGun1 _asheist_data false)
              (Variables|/Game/Blueprints/HeistData.HeistData_C|SetGun2 _asheist_data false)
              (Variables|/Game/Blueprints/HeistData.HeistData_C|SetGun3 _asheist_data false)
              (Variables|/Game/Blueprints/HeistData.HeistData_C|SetGun4 _asheist_data false)
              (Variables|/Game/Blueprints/HeistData.HeistData_C|SetAccessCard _asheist_data false)
              (Variables|/Game/Blueprints/HeistData.HeistData_C|SetFirstSafe _asheist_data false)
              (Variables|/Game/Blueprints/HeistData.HeistData_C|SetHostages _asheist_data 0)
              (UserInterface|Viewport|AddtoViewport _returnvalue_4 0)))))
      (else
        (Variables|Default|SetTimeToExit 0.0)
        (Widget|RemovefromParent _returnvalue_3)))))

(event OnComponentEndOverlap(Box)
  (params (OverlappedComponent :type Primitive%20Component%20Object%20Reference) (OtherActor :type Actor%20Object%20Reference) (OtherComp :type Primitive%20Component%20Object%20Reference) (OtherBodyIndex :type Integer))
  (Utilities|Casting|CastToFirstPersonCharacter OtherActor)
  (Variables|Default|SetLeaving false))

(event OnComponentBeginOverlap(Box1)
  (params (OverlappedComponent :type Primitive%20Component%20Object%20Reference) (OtherActor :type Actor%20Object%20Reference) (OtherComp :type Primitive%20Component%20Object%20Reference) (OtherBodyIndex :type Integer) (bFromSweep :type Boolean) (SweepResult :type Hit%20Result%20Structure%20%28by%20ref%29))
  (bind _asmoney_bag (Utilities|Casting|CastToMoneyBag OtherActor))
  (if (Variables|/Game/Blueprints/MoneyBag.MoneyBag_C|GetEarned _asmoney_bag)
    (Variables|/Game/Blueprints/MoneyBag.MoneyBag_C|SetEarned _asmoney_bag false)
    (Variables|Default|SetHasMoney true)
    (bind _output_get (Variables|Default|SetMoneyGained (+ 5000 (Variables|Default|GetMoneyGained))))
    (Variables|Default|SetHelicopterMoney _output_get)
    (bind _returnvalue (UserInterface|CreateWidget "/Game/Widgets/MoneyEarned.MoneyEarned_C"))
    (Variables|/Game/Widgets/MoneyEarned.MoneyEarned_C|SetCash _returnvalue 5000)
    (UserInterface|Viewport|AddtoViewport _returnvalue 0)
    (Development|PrintString "Money Earned" true true "(R=0.000000,G=0.660000,B=1.000000,A=1.000000)" 5.0)))

(event Custom|Flying
  (Variables|Default|SetEscape true)
  (Viewport|RemoveAllWidgets)
  (bind _asfirst_person_character (Utilities|Casting|CastToFirstPersonCharacter (Game|GetPlayerCharacter 0)))
  (Input|DisableInput _asfirst_person_character 0)
  (bind _outactors (Actor|GetAllActorsOfClass "/Game/Blueprints/MoneyBag.MoneyBag_C"))
  (Actor|DestroyActor _outactors)
  (Game|Player|SetViewTargetwithBlend (Game|GetPlayerController 0) self 1.0 "VTBlend_Linear" 0.0 false)
  (Utilities|FlowControl|Sequence
    (:then_0
      (Components|MoveComponentTo (Variables|Default|GetSM_helicopter_uh_body) "5000.000000,500.000000,8000.000000" "-30.000000, 0, 0" false false 7.0 false)
      (bind _returnvalue (UserInterface|CreateWidget "/Game/Blueprints/UI/JobComplete.JobComplete_C"))
      (UserInterface|Viewport|AddtoViewport _returnvalue 0)
      (Game|SetGamePaused true))
    (:then_1
      (Components|MoveComponentTo (Variables|Default|GetCamera) "2000.000000, 0, 0" "0,180.000000, 0" false false 2.0 false))))

(event Custom|Begin
  (bind _cylinder (Variables|Default|GetCylinder))
  (bind _sm_helicopter_uh_body (Variables|Default|GetSM_helicopter_uh_body))
  (Utilities|FlowControl|Sequence
    (:then_0
      (Transformation|SetRelativeRotation _cylinder (Math|Rotator|MakeRotator 0.0 0.0 (+ (.yaw (Variables|/Script/Engine.SceneComponent|GetRelativeRotation _cylinder)) 25.0)) false false :!label _label)
      (Utilities|FlowControl|Delay 1e-06)
      (goto _label))
    (:then_1
      (bind _output_get (Variables|Default|SetSpin (+ (Variables|Default|GetSpin) 2e+01) :!label _label_2))
      (Transformation|SetRelativeRotation (Variables|Default|GetCylinder1) (Math|Rotator|MakeRotator 9e+01 _output_get 0.0) false false)
      (Utilities|FlowControl|Delay 1e-06)
      (goto _label_2))
    (:then_2
      (Components|MoveComponentTo _sm_helicopter_uh_body "-100.000000, 0, 0" "10.000000, 0, 0" false false 6.0 false)
      (Components|MoveComponentTo _sm_helicopter_uh_body "0, 0,10.000000" "-2.000000, 0, 0" false false 0.5 false)
      (Components|MoveComponentTo _sm_helicopter_uh_body "0, 0, 0" "0, 0, 0" true false 1.0 false))
    (:then_3
      (Components|Activation|SetActive (Variables|Default|GetHelicopterSoundEffect) true false))))

(fn ConstructionScript)