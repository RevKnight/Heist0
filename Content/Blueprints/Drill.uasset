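; Drill actor that gradually breaks open a Safe and can stall along the way.
; The Door event starts or restarts a delayed loop that builds progress, with a rising random chance to stop and turn on its particle system.
; Past the threshold, it calls BrokenOpen on the first Safe found and destroys itself.
; BeginPlay also enters the loop if already working; the cylinder spin logic is never triggered.
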(event EventBeginPlay
  (if (Variables|Default|GetWorking) :!label _label
    (Utilities|FlowControl|Sequence
      (:then_0
        (bind _output_get (Variables|Default|SetBreakingIn (+ (Variables|Default|GetBreakingIn) 0.01)))
        (Utilities|FlowControl|Delay 0.1)
        (if (<= _output_get 0.8)
          (if (Math|Random|RandomBoolwithWeight (/ _output_get 1e+01))
            (Variables|Default|SetWorking false)
            (Components|Activation|SetActive (Variables|Default|GetParticleSystem) true false)
            (else
              (goto _label)))
          (else
            (Development|PrintString "Open")
            (bind _outactors (Actor|GetAllActorsOfClass "/Game/Blueprints/Safe.Safe_C"))
            (bind _assafe (Utilities|Casting|CastToSafe (Utilities|Array|Get(acopy) _outactors)))
            (Default|BrokenOpen _assafe)
            (Actor|DestroyActor)))))))

(event EventDoor
  (if (not (Variables|Default|GetWorking))
    (Variables|Default|SetWorking true)
    (Components|Activation|SetActive (Variables|Default|GetParticleSystem) false false)
    (if (Variables|Default|GetWorking) :!label _label
      (Utilities|FlowControl|Sequence
        (:then_0
          (bind _output_get (Variables|Default|SetBreakingIn (+ (Variables|Default|GetBreakingIn) 0.01)))
          (Utilities|FlowControl|Delay 0.1)
          (if (<= _output_get 0.8)
            (if (Math|Random|RandomBoolwithWeight (/ _output_get 1e+01))
              (Variables|Default|SetWorking false)
              (Components|Activation|SetActive (Variables|Default|GetParticleSystem) true false)
              (else
                (goto _label)))
            (else
              (Development|PrintString "Open")
              (bind _outactors (Actor|GetAllActorsOfClass "/Game/Blueprints/Safe.Safe_C"))
              (bind _assafe (Utilities|Casting|CastToSafe (Utilities|Array|Get(acopy) _outactors)))
              (Default|BrokenOpen _assafe)
              (Actor|DestroyActor))))))))

(fn ConstructionScript)