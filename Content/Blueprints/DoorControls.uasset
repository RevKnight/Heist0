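; Lockable door for a heist game, toggled open and closed by the Door event.
; When locked, it checks AccessCard on the HeistData game instance, either unlocking itself and proceeding or playing a sound and rattling the handle.
; A FlipFlop alternates chained MoveComponentTo animations that turn the handle (Cube2) and swing the panel (Cube) to the Opened yaw or back, with audio.
; A DoOnce guards the opening sequence until it finishes.
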(event EventDoor
  (if (Variables|Default|GetCan%20be%20opened) :!label _label
    (Utilities|FlowControl|FlipFlop
      (:A
        (Utilities|FlowControl|DoOnce false :!label _label_2
          (:Completed
            (Components|Activation|SetActive (Variables|Default|GetAudio) true false)
            (Components|MoveComponentTo (Variables|Default|GetCube2) "86.881744,-5.000000,90.000015" "-45.000000,180.000000, 0" false true 0.3 true)
            (Components|MoveComponentTo (Variables|Default|GetCube) "-142.000000,10.000000, 0" (Math|Rotator|MakeRotator 0.0 0.0 (Variables|Default|GetOpened)) false true 0.75 true)
            (Components|MoveComponentTo (Variables|Default|GetCube2) "86.881744,-5.000000,90.000000" "0.000000,180.000000, 0" false true 0.3 true)
            (goto _label_2 Reset))))
      (:B
        (Components|MoveComponentTo (Variables|Default|GetCube) "-142.000000,10.000000, 0" "0, 0, 0" false true 0.75 true)
        (Components|MoveComponentTo (Variables|Default|GetCube2) "86.881744,-5.000000,90.000000" "-10.000000,180.000000, 0" false true 0.1 true)
        (Utilities|FlowControl|Sequence
          (:then_0
            (Components|MoveComponentTo (Variables|Default|GetCube2) "86.881744,-5.000000,90.000000" "0.000000,180.000000, 0" false true 0.3 true))
          (:then_1
            (Utilities|FlowControl|Delay 0.1)
            (Components|Activation|SetActive (Variables|Default|GetAudio1) true false)))))
    (else
      (bind _asheist_data (Utilities|Casting|CastToHeistData (Game|GetGameInstance)))
      (if (Variables|/Game/Blueprints/HeistData.HeistData_C|GetAccessCard _asheist_data)
        (Variables|Default|SetCan%20be%20opened true)
        (goto _label)
        (else
          (Components|Activation|SetActive (Variables|Default|GetAudio2) true false)
          (Components|MoveComponentTo (Variables|Default|GetCube2) "86.881744,-5.000000,90.000000" "-80.000000,180.000000, 0" false false 0.2 false)
          (Components|MoveComponentTo (Variables|Default|GetCube2) "86.881744,-5.000000,90.000000" "0,180.000000, 0" false false 1.0 false)
          (Components|MoveComponentTo (Variables|Default|GetCube2) "86.881744,-5.000000,90.000000" "-70.000000,180.000000, 0" false false 0.3 false)
          (Components|MoveComponentTo (Variables|Default|GetCube2) "86.881744,-5.000000,90.000000" "-30.000000,180.000000, 0" false false 0.2 false)
          (Components|MoveComponentTo (Variables|Default|GetCube2) "86.881744,-5.000000,90.000000" "-50.000000,180.000000, 0" false false 0.2 false)
          (Components|MoveComponentTo (Variables|Default|GetCube2) "86.881744,-5.000000,90.000000" "0,180.000000, 0" false false 0.6 false))))))

(fn ConstructionScript)