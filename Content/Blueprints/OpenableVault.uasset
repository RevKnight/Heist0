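; Openable vault that the player can attach a drill to and that later swings open.
; Door casts the player to FirstPersonCharacter and, through a resettable DoOnce, spawns a scaled Drill below the vault's origin, flagged as a vault drill, when DrillBomb is zero.
; SwingOpen rotates and slides one door mesh over time with MoveComponentTo.
; A mirrored move for a second mesh is left unconnected.
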(event Custom|Reset
  (bind _returnvalue (Transformation|GetActorTransform))
  (Utilities|FlowControl|DoOnce false) ; enters at Reset
)

(event Custom|SwingOpen
  (Components|MoveComponentTo (Variables|Default|GetStaticMeshComponent01) "57.849998,23.200001, 0" "0,-90.000000, 0" false false 5.0 true))

(event EventDoor
  (bind _returnvalue (Transformation|GetActorTransform))
  (bind _asfirst_person_character (Utilities|Casting|CastToFirstPersonCharacter (Game|GetPlayerCharacter 0)))
  (Utilities|FlowControl|DoOnce false
    (:Completed
      (switch int (Variables|/Game/FirstPersonBP/Blueprints/FirstPersonCharacter.FirstPersonCharacter_C|GetDrill/Bomb _asfirst_person_character)
        (:0
          (bind _returnvalue_2 (Game|SpawnActorfromClass "/Game/Blueprints/Drill.Drill_C" (Math|Transform|MakeTransform (- (.location _returnvalue) "0, 0,160.000000") (.rotation _returnvalue) "1.200000,1.200000,1.200000") "Undefined" 0 0))
          (Variables|/Game/Blueprints/Drill.Drill_C|SetVault _returnvalue_2 true))))))

(fn ConstructionScript)