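; Slot machine gamble that the player triggers through the Door event while carrying, giving up the carried state and restoring walk speed.
; A DoOnce-guarded pull moves Cube1 and picks one of five random branches, spinning three cylinder reels through tick-length Delay loops.
; One branch awards a random gun, another a HeistData bomb, and the rest nothing, before the machine resets.
; A 5000 cash charge exists but is never wired up.
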(event EventDoor
  (bind _asfirst_person_character (Utilities|Casting|CastToFirstPersonCharacter (Game|GetPlayerCharacter 0)))
  (if (Variables|/Game/FirstPersonBP/Blueprints/FirstPersonCharacter.FirstPersonCharacter_C|GetCarrying _asfirst_person_character)
    (Variables|/Game/FirstPersonBP/Blueprints/FirstPersonCharacter.FirstPersonCharacter_C|SetCarrying _asfirst_person_character false)
    (Variables|/Script/Engine.CharacterMovementComponent|SetMaxWalkSpeed (Variables|/Script/Engine.Character|GetCharacterMovement _asfirst_person_character) 6e+02)
    (Utilities|FlowControl|DoOnce false :!label _label
      (:Completed
        (Components|MoveComponentTo (Variables|Default|GetCube1) "0,-45.000000,40.000000" "-50.000000, 0, 0" false false 0.2 false)
        (switch int (Math|Random|RandomIntegerinRange 0 4)
          (:0
            (Utilities|FlowControl|Sequence :!label _label_2
              (:then_0
                (bind _output_get (Variables|Default|SetWheel1 (Math|Rotator|MakeRotator 9e+01 (+ (.pitch (Variables|Default|GetWheel1)) (Math|Random|RandomFloatinRange 1.0 1e+01)) 0.0)))
                (Transformation|SetRelativeRotation (Variables|Default|GetCylinder) _output_get false false)
                (Utilities|FlowControl|Delay 1e-05)
                (if (<= (.pitch (Variables|Default|GetWheel1)) 1.4e+03)
                  (goto _label_2)
                  (else
                    (bind _asfirst_person_character_2 (Utilities|Casting|CastToFirstPersonCharacter (Game|GetPlayerCharacter 0)))
                    (switch int (Math|Random|RandomIntegerinRange 0 2)
                      (:0
                        (Variables|/Game/FirstPersonBP/Blueprints/FirstPersonCharacter.FirstPersonCharacter_C|SetGunInventory _asfirst_person_character_2 2))
                      (:1
                        (Variables|/Game/FirstPersonBP/Blueprints/FirstPersonCharacter.FirstPersonCharacter_C|SetGunInventory _asfirst_person_character_2 4))
                      (:2
                        (Variables|/Game/FirstPersonBP/Blueprints/FirstPersonCharacter.FirstPersonCharacter_C|SetGunInventory _asfirst_person_character_2 6)))
                    (Default|SwitchedWeapons _asfirst_person_character_2)
                    (Utilities|FlowControl|Delay 2.0 :!label _label_3)
                    (Transformation|SetRelativeRotation (Variables|Default|GetCylinder) "-30.000000,180.000000,270.000000" false false)
                    (Transformation|SetRelativeRotation (Variables|Default|GetCylinder1) "90.000000,355.000000,445.000000" false false)
                    (Transformation|SetRelativeRotation (Variables|Default|GetCylinder2) "-35.000000,0.000000,90.000000" false false)
                    (Components|MoveComponentTo (Variables|Default|GetCube1) "0,-45.000000,40.000000" "0, 0, 0" false false 0.4 false)
                    (Variables|Default|SetRandom true)
                    (Variables|Default|SetWheel1 "0, 0, 0")
                    (Variables|Default|SetWheel2 "200.000000, 0, 0")
                    (Variables|Default|SetWheel3 "700.000000, 0, 0")
                    (goto _label Reset))))
              (:then_1
                (bind _output_get_2 (Variables|Default|SetWheel1 (Math|Rotator|MakeRotator 9e+01 (+ (.pitch (Variables|Default|GetWheel1)) (Math|Random|RandomFloatinRange 1.0 1e+01)) 0.0)))
                (Transformation|SetRelativeRotation (Variables|Default|GetCylinder1) _output_get_2 false false))
              (:then_2
                (bind _output_get_3 (Variables|Default|SetWheel1 (Math|Rotator|MakeRotator 9e+01 (+ (.pitch (Variables|Default|GetWheel1)) (Math|Random|RandomFloatinRange 1.0 1e+01)) 0.0)))
                (Transformation|SetRelativeRotation (Variables|Default|GetCylinder2) _output_get_3 false false))))
          (:1
            (Utilities|FlowControl|Sequence :!label _label_4
              (:then_0
                (bind _output_get_4 (Variables|Default|SetWheel1 (Math|Rotator|MakeRotator 9e+01 (+ (.pitch (Variables|Default|GetWheel1)) (Math|Random|RandomFloatinRange 1.0 1e+01)) 0.0)))
                (Transformation|SetRelativeRotation (Variables|Default|GetCylinder) _output_get_4 false false)
                (Utilities|FlowControl|Delay 1e-05)
                (if (<= (.pitch (Variables|Default|GetWheel1)) 1.3e+03)
                  (goto _label_4)
                  (else
                    (bind _asheist_data (Utilities|Casting|CastToHeistData (Game|GetGameInstance)))
                    (Variables|/Game/Blueprints/HeistData.HeistData_C|SetBomb _asheist_data (+ (Variables|/Game/Blueprints/HeistData.HeistData_C|GetBomb _asheist_data) 1))
                    (goto _label_3))))
              (:then_1
                (bind _output_get_5 (Variables|Default|SetWheel1 (Math|Rotator|MakeRotator 9e+01 (+ (.pitch (Variables|Default|GetWheel1)) (Math|Random|RandomFloatinRange 1.0 1e+01)) 0.0)))
                (Transformation|SetRelativeRotation (Variables|Default|GetCylinder1) _output_get_5 false false))
              (:then_2
                (bind _output_get_6 (Variables|Default|SetWheel1 (Math|Rotator|MakeRotator 9e+01 (+ (.pitch (Variables|Default|GetWheel1)) (Math|Random|RandomFloatinRange 1.0 1e+01)) 0.0)))
                (Transformation|SetRelativeRotation (Variables|Default|GetCylinder2) _output_get_6 false false))))
          (:2
            (Utilities|FlowControl|Sequence :!label _label_5
              (:then_0
                (bind _output_get_7 (Variables|Default|SetWheel1 (Math|Rotator|MakeRotator 9e+01 (+ (.pitch (Variables|Default|GetWheel1)) (Math|Random|RandomFloatinRange 1.0 1e+01)) 0.0)))
                (Transformation|SetRelativeRotation (Variables|Default|GetCylinder) _output_get_7 false false)
                (Utilities|FlowControl|Delay 1e-05)
                (if (<= (.pitch (Variables|Default|GetWheel1)) 925.0)
                  (goto _label_5)
                  (else
                    (goto _label_3))))
              (:then_1
                (bind _output_get_8 (Variables|Default|SetWheel1 (Math|Rotator|MakeRotator 9e+01 (+ (.pitch (Variables|Default|GetWheel1)) (Math|Random|RandomFloatinRange 1.0 1e+01)) 0.0)))
                (Transformation|SetRelativeRotation (Variables|Default|GetCylinder1) _output_get_8 false false))
              (:then_2
                (bind _output_get_9 (Variables|Default|SetWheel1 (Math|Rotator|MakeRotator 9e+01 (+ (.pitch (Variables|Default|GetWheel1)) (Math|Random|RandomFloatinRange 1.0 1e+01)) 0.0)))
                (Transformation|SetRelativeRotation (Variables|Default|GetCylinder2) _output_get_9 false false))))
          (:3
            (Utilities|FlowControl|Sequence :!label _label_6
              (:then_0
                (bind _output_get_10 (Variables|Default|SetWheel1 (Math|Rotator|MakeRotator 9e+01 (+ (.pitch (Variables|Default|GetWheel1)) 2e+01) 0.0)))
                (Transformation|SetRelativeRotation (Variables|Default|GetCylinder) _output_get_10 false false)
                (Utilities|FlowControl|Delay 1e-05)
                (Utilities|FlowControl|Sequence
                  (:then_0
                    (if (Variables|Default|GetRandom)
                      (goto _label_6)
                      (else
                        (goto _label_3))))
                  (:then_1
                    (Utilities|FlowControl|Delay 1.0)
                    (Variables|Default|SetRandom false))))
              (:then_1
                (bind _output_get_11 (Variables|Default|SetWheel2 (Math|Rotator|MakeRotator 9e+01 (+ (.pitch (Variables|Default|GetWheel2)) 2e+01) 0.0)))
                (Transformation|SetRelativeRotation (Variables|Default|GetCylinder1) _output_get_11 false false))
              (:then_2
                (bind _output_get_12 (Variables|Default|SetWheel3 (Math|Rotator|MakeRotator 9e+01 (+ (.pitch (Variables|Default|GetWheel3)) 2e+01) 0.0)))
                (Transformation|SetRelativeRotation (Variables|Default|GetCylinder2) _output_get_12 false false))))
          (:4
            (goto _label_6)))))))

(fn ConstructionScript)