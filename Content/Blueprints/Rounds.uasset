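; Rounds tracks state for police assault waves.
; From BeginPlay it polls the first SpawnPoint every half second, copying its HitPoints into PoliceHealth.
; Count events adjust SpawnNumber, with decrements flagging WaveIncrease while the result is at least -5.
; WaveCount fires the game mode HUD's PoliceAssault through a DoOnce, whose reset sits in disconnected wave-widget logic.
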(event Custom|PoliceCountNegative
  (Variables|Default|SetSpawnNumber (- (Variables|Default|GetSpawnNumber) 1))
  (if (>= (Variables|Default|GetSpawnNumber) -5)
    (Variables|Default|SetWaveIncrease true)))

(event Custom|WaveCount
  (Utilities|FlowControl|DoOnce false
    (:Completed
      (bind _asfirst_person_game_mode (Utilities|Casting|CastToFirstPersonGameMode (Game|GetGameMode)))
      (Default|PoliceAssault (Variables|/Game/FirstPersonBP/Blueprints/FirstPersonGameMode.FirstPersonGameMode_C|GetHUDRef _asfirst_person_game_mode)))))

(event Custom|PoliceCountPositive
  (Variables|Default|SetSpawnNumber (+ (Variables|Default|GetSpawnNumber) 1)))

(event EventBeginPlay
  (bind _outactors (Actor|GetAllActorsOfClass "/Game/Blueprints/SpawnPoint.SpawnPoint_C" :!label _label))
  (bind _asspawn_point (Utilities|Casting|CastToSpawnPoint (Utilities|Array|Get(acopy) _outactors)))
  (Variables|Default|SetPoliceHealth (Variables|/Game/Blueprints/SpawnPoint.SpawnPoint_C|GetHitPoints _asspawn_point))
  (Utilities|FlowControl|Delay 0.5)
  (goto _label))

(fn ConstructionScript)