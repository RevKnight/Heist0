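; Vent input actor that takes in money bags and hands them to a linked out door.
; A BP_MoneyBag overlapping the Box is passed to OutDoor through OutBagMessage, then destroyed after a short delay.
; BeginPlay and Hit share one chain that turns on physics for the Cover and removes it a few seconds later.
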(event OnComponentBeginOverlap(Box)
  (params (OverlappedComponent :type Primitive%20Component%20Object%20Reference) (OtherActor :type Actor%20Object%20Reference) (OtherComp :type Primitive%20Component%20Object%20Reference) (OtherBodyIndex :type Integer) (bFromSweep :type Boolean) (SweepResult :type Hit%20Result%20Structure%20%28by%20ref%29))
  (bind _asbp_money_bag (Utilities|Casting|CastToBP_MoneyBag OtherActor))
  (Class|BPIVentCommunication|OutBag(Message) (Variables|Default|GetOutDoor) _asbp_money_bag)
  (Utilities|FlowControl|Delay 0.2)
  (Actor|DestroyActor _asbp_money_bag))

(event Collision|EventActorBeginOverlap
  (params (OtherActor :type Actor%20Object%20Reference)))

(event EventTick
  (params (DeltaSeconds :type Float%20%28single-precision%29)))

(event EventHit
  (Physics|SetSimulatePhysics (Variables|Default|GetCover) true)
  (Utilities|FlowControl|Delay 3.0)
  (Components|DestroyComponent (Variables|Default|GetCover)))

(event EventBeginPlay
  (Physics|SetSimulatePhysics (Variables|Default|GetCover) true)
  (Utilities|FlowControl|Delay 3.0)
  (Components|DestroyComponent (Variables|Default|GetCover)))

(fn ConstructionScript)