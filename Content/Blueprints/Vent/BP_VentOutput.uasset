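; Vent exit that drops its cover and launches money bags out of the duct.
; On BeginPlay or a Hit, the cover starts simulating physics and is destroyed after a short delay.
; OutBag spawns a new bag of the passed MoneyBag's class at the Arrow, then applies a velocity-change impulse along the arrow's forward vector, scaled by PushPower.
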(event Collision|EventActorBeginOverlap
  (params (OtherActor :type Actor%20Object%20Reference)))

(event EventTick
  (params (DeltaSeconds :type Float%20%28single-precision%29)))

(event EventOutBag
  (params (MoneyBag :type BP%20Money%20Bag%20Object%20Reference))
  (bind _returnvalue (Game|SpawnActorfromClass (Utilities|GetClass MoneyBag) (Math|Transform|MakeTransform (Transformation|GetSocketLocation (Variables|Default|GetArrow) "None")) "Undefined" 0 0))
  (bind _output_get (Variables|Default|SetMoney%20Bag _returnvalue))
  (Physics|AddImpulse (Variables|/Game/Blueprints/Vent/BP_MoneyBag.BP_MoneyBag_C|GetCube _output_get) (* (Math|Vector|GetForwardVector (Variables|Default|GetArrow)) (Variables|Default|GetPushPower)) "None" true))

(event EventHit
  (Physics|SetSimulatePhysics (Variables|Default|GetCover) true)
  (Utilities|FlowControl|Delay 3.0)
  (Components|DestroyComponent (Variables|Default|GetCover)))

(event EventBeginPlay
  (Physics|SetSimulatePhysics (Variables|Default|GetCover) true)
  (Utilities|FlowControl|Delay 3.0)
  (Components|DestroyComponent (Variables|Default|GetCover)))

(fn ConstructionScript)