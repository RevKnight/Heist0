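; Weapon sight attachment Blueprint that controls its lens rendering and the visibility of its mounting pieces.
; Two events hand one lens render target to either the behind-lens or reflection capture, clearing the other.
; Lens reflection and dust are toggled through a dynamic material instance on the sight mesh.
; An adapter ID reveals a RIS adapter, high RIS adapter or Strike ironsight, with a separate event hiding all three.
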(event Custom|ActivateBackRenderTexture
  (Variables|/Script/Engine.SceneCaptureComponent2D|SetTextureTarget (Variables|Default|GetLensBehindCaptureComponent) "/Game/Weapons/Textures/Attachments/LensRenderToTexture.LensRenderToTexture")
  (Variables|/Script/Engine.SceneCaptureComponent2D|SetTextureTarget (Variables|Default|GetLensReflectionCapture) 0))

(event Custom|ActivateForwardRenderTexture
  (Variables|/Script/Engine.SceneCaptureComponent2D|SetTextureTarget (Variables|Default|GetLensBehindCaptureComponent) 0)
  (Variables|/Script/Engine.SceneCaptureComponent2D|SetTextureTarget (Variables|Default|GetLensReflectionCapture) "/Game/Weapons/Textures/Attachments/LensRenderToTexture.LensRenderToTexture"))

(event Custom|DisableLensReflection
  (bind _returnvalue (Rendering|Material|CreateDynamicMaterialInstance (Variables|Default|GetSight) 1 (Variables|Default|GetLensMaterial) :!class /Script/Engine.PrimitiveComponent))
  (Rendering|Material|SetScalarParameterValue _returnvalue "Dust&ReflectionPower" 0.0 :!class /Script/Engine.MaterialInstanceDynamic))

(event Custom|EnableLensReflection
  (bind _returnvalue (Rendering|Material|CreateDynamicMaterialInstance (Variables|Default|GetSight) 1 (Variables|Default|GetLensMaterial) :!class /Script/Engine.PrimitiveComponent))
  (Rendering|Material|SetScalarParameterValue _returnvalue "Dust&ReflectionPower" 1.0 :!class /Script/Engine.MaterialInstanceDynamic))

(event Custom|ShowRisAdapter
  (params (AdapterID :type Integer))
  (switch int AdapterID
    (:0
      (Rendering|SetVisibility (Variables|Default|GetRIS_Adapter) true false))
    (:1
      (Rendering|SetVisibility (Variables|Default|GetStrike_Ironsight) true false))
    (:2
      (Rendering|SetVisibility (Variables|Default|GetRIS_Adapter_high) true false))))

(event Custom|ClearAllAdapters
  (Rendering|SetVisibility (Variables|Default|GetRIS_Adapter) false false)
  (Rendering|SetVisibility (Variables|Default|GetStrike_Ironsight) false false)
  (Rendering|SetVisibility (Variables|Default|GetRIS_Adapter_high) false false))

(event EventBeginPlay)

(event EventActorBeginOverlap
  (params (OtherActor :type Actor%20Object%20Reference)))

(event EventTick
  (params (DeltaSeconds :type Float%20%28single-precision%29)))

(fn ConstructionScript)