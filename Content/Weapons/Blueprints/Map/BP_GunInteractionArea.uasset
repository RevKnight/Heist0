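; Gun pickup pedestal area that lets the player interact to switch to the weapon it holds.
; Box overlap toggles interaction, recolors the caption, spawns or destroys a light actor, and sets the player's shop-interaction flag, registering this area on begin.
; SetNewVar pushes this gun's mesh, sight, animations, ID and FX to the stored character.
; Construction creates a dynamic pedestal material, and TestActive exposes the interaction state.
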(event OnComponentEndOverlap(Box)
  (params (OverlappedComponent :type Primitive%20Component%20Object%20Reference) (OtherActor :type Actor%20Object%20Reference) (OtherComp :type Primitive%20Component%20Object%20Reference) (OtherBodyIndex :type Integer))
  ;[1 1 1] Disable interaction when overaly end
  ;;[1 1 1] Set label color to default
  (Rendering|Components|TextRender|SetTextRenderColor (Variables|/Script/Engine.TextRenderActor|GetTextRender (Variables|Default|GetCaption)) (Math|Conversions|ToColor(LinearColor) (Variables|Default|GetDefaultColor)))
  (Variables|Default|SetInteractionEnabled false)
  (bind _asgbplayer_main (Utilities|Casting|CastToGBPlayerMain OtherActor))
  ;;[1 1 1] Remove light point
  (Actor|DestroyActor (Variables|Default|GetLightSpawned))
  (Variables|/Game/Game_Content/GameFramework/GBPlayerMain.GBPlayerMain_C|SetbEnableShopInteraction _asgbplayer_main false))

(event OnComponentBeginOverlap(Box)
  (params (OverlappedComponent :type Primitive%20Component%20Object%20Reference) (OtherActor :type Actor%20Object%20Reference) (OtherComp :type Primitive%20Component%20Object%20Reference) (OtherBodyIndex :type Integer) (bFromSweep :type Boolean) (SweepResult :type Hit%20Result%20Structure%20%28by%20ref%29))
  ;[1 1 1] Enable interaction when overaly begin
  (Variables|Default|SetInteractionEnabled true)
  (bind _asgbplayer_main (Utilities|Casting|CastToGBPlayerMain (Game|GetPlayerCharacter 0)))
  ;;[1 1 1] Set label color
  (Rendering|Components|TextRender|SetTextRenderColor (Variables|/Script/Engine.TextRenderActor|GetTextRender (Variables|Default|GetCaption)) (Math|Conversions|ToColor(LinearColor) (Variables|Default|GetEnabledColor)))
  ;;[1 1 1] Spawn LightPoint actor
  (bind _returnvalue (Game|SpawnActorfromClass "/Game/Weapons/Blueprints/Map/BP_LightActor.BP_LightActor_C" (Transformation|GetWorldTransform (Variables|Default|GetLightPosition)) "Undefined" 0 0))
  (Variables|Default|SetLightSpawned _returnvalue)
  (Variables|/Game/Game_Content/GameFramework/GBPlayerMain.GBPlayerMain_C|SetInteractionArea _asgbplayer_main self)
  (Variables|/Game/Game_Content/GameFramework/GBPlayerMain.GBPlayerMain_C|SetbEnableShopInteraction _asgbplayer_main true)
  (Variables|Default|SetCharacter_reference _asgbplayer_main))

(event Custom|SetNewVar
  ;[1 1 1] Set gun vars to mainCharacter
  (Default|SetNewGunStuff (Variables|Default|GetCharacter_reference) (Variables|Default|GetGunSkeletalMesh) (Variables|Default|GetIronSight) (Variables|Default|GetGun_FireMontage) (Variables|Default|GetGun_IdleAnim) (Variables|Default|GetGun_ReloadMontage) (Variables|Default|GetGun_AnimBlueprint) (Variables|Default|GetGun_ADSFireMontage) (Variables|Default|GetArms_FireMontage) (Variables|Default|GetArms_ADSFireMontage) (Variables|Default|GetArms_ReloadMontage) (Variables|Default|GetArms_RaiseMontage) (Variables|Default|GetArms_LowerMontage) (Variables|Default|GetGunId) (Variables|Default|GetFX)))

(fn ConstructionScript
  (bind _returnvalue (Rendering|Material|CreateDynamicMaterialInstance (Variables|/Script/Engine.StaticMeshActor|GetStaticMeshComponent (Variables|Default|GetPedestal)) 0 0 :!class /Script/Engine.PrimitiveComponent))
  (LocalVariables|SetPedestalMaterialInstance _returnvalue))

(fn TestActive
  (return (Variables|Default|GetInteractionEnabled)))