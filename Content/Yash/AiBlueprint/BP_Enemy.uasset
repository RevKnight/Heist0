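; BP_Enemy is an AI enemy that takes projectile damage and shows a health bar when the first-person character is near.
; On BeginPlay it passes itself as OwnerHealth to the AI_HealthBarWidget in its HeathBar component.
; Sphere overlaps with the FirstPersonCharacter toggle that bar's visibility.
; Capsule hits by a FirstPersonProjectile subtract its Damage from Health, with no clamp or death handling here.
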(event OnComponentBeginOverlap(Sphere)
  (params (OverlappedComponent :type Primitive%20Component%20Object%20Reference) (OtherActor :type Actor%20Object%20Reference) (OtherComp :type Primitive%20Component%20Object%20Reference) (OtherBodyIndex :type Integer) (bFromSweep :type Boolean) (SweepResult :type Hit%20Result%20Structure%20%28by%20ref%29))
  (Utilities|Casting|CastToFirstPersonCharacter OtherActor)
  (Rendering|SetVisibility (Variables|Default|GetHeathBar) true false))

(event OnComponentEndOverlap(Sphere)
  (params (OverlappedComponent :type Primitive%20Component%20Object%20Reference) (OtherActor :type Actor%20Object%20Reference) (OtherComp :type Primitive%20Component%20Object%20Reference) (OtherBodyIndex :type Integer))
  (Utilities|Casting|CastToFirstPersonCharacter OtherActor)
  (Rendering|SetVisibility (Variables|Default|GetHeathBar) false false))

(event OnComponentHit(CapsuleComponent)
  (params (HitComponent :type Primitive%20Component%20Object%20Reference) (OtherActor :type Actor%20Object%20Reference) (OtherComp :type Primitive%20Component%20Object%20Reference) (NormalImpulse :type Vector :default "0, 0, 0") (Hit :type Hit%20Result%20Structure%20%28by%20ref%29))
  (bind _asfirst_person_projectile (Utilities|Casting|CastToFirstPersonProjectile OtherActor))
  (Variables|Default|SetHealth (- (Variables|Default|GetHealth) (Variables|/Game/FirstPersonBP/Blueprints/FirstPersonProjectile.FirstPersonProjectile_C|GetDamage _asfirst_person_projectile))))

(event EventBeginPlay
  (bind _asai_health_bar_widget (Utilities|Casting|CastToAI_HealthBarWidget (UserInterface|GetUserWidgetObject (Variables|Default|GetHeathBar))))
  (Variables|/Game/Yash/AiBlueprint/AI_HealthBarWidget.AI_HealthBarWidget_C|SetOwnerHealth _asai_health_bar_widget self))

(fn ConstructionScript)