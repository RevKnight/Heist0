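; BP_Door02A is a configurable door prop from the SovietDoors folder, posed at construction with no active runtime logic.
; The construction script yaws the Door02A component by the Door variable.
; It also slides the Door02AADD01 and StaticMesh components along local X by DoorAdd01 and DoorAdd02 respectively.
; The event graph holds only disabled placeholder events, so the script provides no interaction or animation.
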(event EventBeginPlay)

(event Collision|EventActorBeginOverlap
  (params (OtherActor :type Actor%20Object%20Reference)))

(event EventTick
  (params (DeltaSeconds :type Float%20%28single-precision%29)))

(fn ConstructionScript
  (Utilities|FlowControl|Sequence
    (:then_0
      (Transformation|AddLocalRotation (Variables|Default|GetDoor02_a) (Math|Rotator|MakeRotator 0.0 0.0 (Variables|Default|GetDoor)) false false))
    (:then_1
      (Transformation|AddLocalOffset (Variables|Default|GetDoor02_a_ADD01) (Math|Vector|MakeVector (Variables|Default|GetDoorAdd01) 0.0 0.0) false false))
    (:then_3
      (Transformation|AddLocalOffset (Variables|Default|GetStaticMesh) (Math|Vector|MakeVector (Variables|Default|GetDoorAdd02) 0.0 0.0) false false))))